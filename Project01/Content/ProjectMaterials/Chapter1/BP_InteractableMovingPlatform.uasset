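; Interactable moving platform actor that slides between its start position and an end marker component when a player interacts with it.
; BeginPlay caches both world locations; the Interact interface calls Move, whose FlipFlop alternates playing and reversing a timeline that lerps the platform's location without sweep.
; When the timeline finishes, a five-second delay triggers an automatic reverse back toward the start.
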(event Custom|Move
  ;[1 1 1] Comment
  (Utilities|FlowControl|FlipFlop
    (:A
      (bind _platformfloattime (Timeline|PlatformTime Play)
        (:Update
          (Transformation|SetWorldLocation (Variables|Default|GetMovingPlatform) (Math|Vector|Lerp(Vector) (Variables|Default|GetStartLocation) (Variables|Default|GetEndLocation) _platformfloattime) false false))
        (:Finished
          (Utilities|FlowControl|Delay 5.0)
          (Timeline|PlatformTime Reverse))))
    (:B
      (Timeline|PlatformTime Reverse))))

(event EventBeginPlay
  ;[1 1 1] Comment
  (Variables|Default|SetStartLocation (Transformation|GetWorldLocation (Variables|Default|GetMovingPlatform)))
  (Variables|Default|SetEndLocation (Transformation|GetWorldLocation (Variables|Default|GetMovingPlatformEnd))))

(fn ConstructionScript)

(fn Interact
  ;[1 1 1] Interact Interface Implementation
  (CallFunction|Move)
  (return true))