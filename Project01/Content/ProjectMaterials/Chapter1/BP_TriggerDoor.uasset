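; BP_TriggerDoor is an interactable door that slides vertically open when a player triggers it.
; A box overlap with the ThirdPersonCharacter shows and hides a text prompt.
; The Interact interface function fires OpenDoor, where a timeline adds a vertical offset to the mesh location cached at BeginPlay.
; The timeline only plays forward, with no closing logic.
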(event OnComponentBeginOverlap(Box)
  (params (OverlappedComponent :type Primitive%20Component%20Object%20Reference) (OtherActor :type Actor%20Object%20Reference) (OtherComp :type Primitive%20Component%20Object%20Reference) (OtherBodyIndex :type Integer) (bFromSweep :type Boolean) (SweepResult :type Hit%20Result%20Structure%20%28by%20ref%29))
  ;[1 1 1] UI Visibility
  (Utilities|Casting|CastToThirdPersonCharacter OtherActor)
  (Rendering|SetVisibility (Variables|Default|GetTextRender) true false))

(event OnComponentEndOverlap(Box)
  (params (OverlappedComponent :type Primitive%20Component%20Object%20Reference) (OtherActor :type Actor%20Object%20Reference) (OtherComp :type Primitive%20Component%20Object%20Reference) (OtherBodyIndex :type Integer))
  ;[1 1 1] UI Visibility
  (Utilities|Casting|CastToThirdPersonCharacter OtherActor)
  (Rendering|SetVisibility (Variables|Default|GetTextRender) false false))

(event Custom|OpenDoor
  ;[1 1 1] Open Door Logic
  (bind _verticaloffset (Timeline|DoorOpeningTimeline Play)
    (:Update
      (Transformation|SetWorldLocation (Variables|Debug|GetStaticMeshComponent) (+ (Variables|Default|GetStartingLocation) (Math|Vector|MakeVector 0.0 0.0 _verticaloffset)) false false))))

(event EventBeginPlay
  ;[1 1 1] Get Starting Location
  (Variables|Default|SetStartingLocation (Transformation|GetWorldLocation (Variables|Debug|GetStaticMeshComponent))))

(fn ConstructionScript)

(fn Interact
  ;[1 1 1] Interact Interface Implementation
  (CallFunction|OpenDoor)
  (return true))