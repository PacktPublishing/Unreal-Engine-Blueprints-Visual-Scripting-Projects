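; BP_QuestDoor is an interactable door that only opens while its linked quest is in progress.
; A box overlap by the player shows or hides a text prompt whose wording follows QuestManager's QuestState.
; The Interact interface calls OpenDoor, which notifies QuestManager and plays a timeline that offsets the mesh vertically from its BeginPlay location.
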(event OnComponentBeginOverlap(Box)
  (params (OverlappedComponent :type Primitive%20Component%20Object%20Reference) (OtherActor :type Actor%20Object%20Reference) (OtherComp :type Primitive%20Component%20Object%20Reference) (OtherBodyIndex :type Integer) (bFromSweep :type Boolean) (SweepResult :type Hit%20Result%20Structure%20%28by%20ref%29))
  (bind _textrender (Variables|Default|GetTextRender))
  ;[1 1 1] UI Visibility
  (Utilities|Casting|CastToThirdPersonCharacter OtherActor)
  (Rendering|SetVisibility (Variables|Default|GetTextRender) true false)
  ;[1 1 1] Change Text based on Quest State
  (switch Utilities|FlowControl|Switch|SwitchonEQuestState (Variables|/Game/Quest-System/QuestManager.QuestManager_C|GetQuestState (Variables|Default|GetQuestManager))
    (:NewEnumerator0
      (Rendering|Components|TextRender|SetText _textrender (Utilities|Text|MakeLiteralText "You need to start <br>a quest first!")))
    (:NewEnumerator1
      (Rendering|Components|TextRender|SetText _textrender (Utilities|Text|MakeLiteralText "Press \"E\" <br>to interact")))))

(event OnComponentEndOverlap(Box)
  (params (OverlappedComponent :type Primitive%20Component%20Object%20Reference) (OtherActor :type Actor%20Object%20Reference) (OtherComp :type Primitive%20Component%20Object%20Reference) (OtherBodyIndex :type Integer))
  (bind _textrender (Variables|Default|GetTextRender))
  ;[1 1 1] UI Visibility
  (Utilities|Casting|CastToThirdPersonCharacter OtherActor)
  (Rendering|SetVisibility (Variables|Default|GetTextRender) false false)
  ;[1 1 1] Change Text based on Quest State
  (switch Utilities|FlowControl|Switch|SwitchonEQuestState (Variables|/Game/Quest-System/QuestManager.QuestManager_C|GetQuestState (Variables|Default|GetQuestManager))
    (:NewEnumerator0
      (Rendering|Components|TextRender|SetText _textrender (Utilities|Text|MakeLiteralText "You need to start <br>a quest first!")))
    (:NewEnumerator1
      (Rendering|Components|TextRender|SetText _textrender (Utilities|Text|MakeLiteralText "Press \"E\" <br>to interact")))))

(event Custom|OpenDoor
  ;[1 1 1] Check if the quest is In Progress
  (switch Utilities|FlowControl|Switch|SwitchonEQuestState (Variables|/Game/Quest-System/QuestManager.QuestManager_C|GetQuestState (Variables|Default|GetQuestManager))
    (:NewEnumerator1
      ;[1 1 1] Notify Quest Manger that Door has been Opened now
      (Default|DoorOpened (Variables|Default|GetQuestManager))
      ;[1 1 1] Open Door Logic
      (bind _verticaloffset (Timeline|DoorOpeningTimeline Play)
        (:Update
          (Transformation|SetWorldLocation (Variables|Debug|GetStaticMeshComponent) (+ (Variables|Default|GetStartingLocation) (Math|Vector|MakeVector 0.0 0.0 _verticaloffset)) false false))))))

(event EventBeginPlay
  ;[1 1 1] Get Starting Location
  (Variables|Default|SetStartingLocation (Transformation|GetWorldLocation (Variables|Debug|GetStaticMeshComponent))))

(fn ConstructionScript)

(fn Interact
  ;[1 1 1] Interact Interface Implementation
  (CallFunction|OpenDoor)
  (return true))