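; BP_Hound is a hound enemy character that bites players and can be killed with silver bullets.
; The construction script loads health, speed, bite distance and regen rate from the EnemiesTable "TypeA" row, and a looping timer regenerates health without a cap.
; Silver bullet hits subtract health, triggering either a multicast impact effect or death through BP_HoundController and delayed destruction.
; Server_Bite applies fixed damage to the first overlapping player.
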(event OnComponentHit(BodyCollision)
  (params (HitComponent :type Primitive%20Component%20Object%20Reference) (OtherActor :type Actor%20Object%20Reference) (OtherComp :type Primitive%20Component%20Object%20Reference) (NormalImpulse :type Vector :default "0, 0, 0") (Hit :type Hit%20Result%20Structure%20%28by%20ref%29))
  ;[1 1 1] Server - Hound (body) Hit
  (Utilities|Casting|CastToSilverBullet OtherActor)
  (bind _output_get (Variables|Default|SetHealth (- (Variables|Default|GetHealth) 25.0)))
  (if (<= _output_get 0.0)
    ;[1 1 1] Server - Hound Death
    (bind _asbp_hound_controller (Utilities|Casting|CastToBP_HoundController (Pawn|GetController)))
    (Default|ServerHoundDie _asbp_hound_controller)
    (Components|DestroyComponent (Variables|Default|GetBodyCollision))
    (Utilities|FlowControl|Delay 1e+01)
    (Actor|DestroyActor)
    (else
      (CallFunction|MulticastSpawnHitEffect (.Location (Collision|BreakHitResult Hit))))))

(event Custom|Multicast_SpawnHitEffect
  (params (HitLocation :type Vector))
  ;[1 1 1] Multicast - Spawn Hit Effect
  (Effects|SpawnEmitteratLocation "/Game/InfinityBladeEffects/Effects/FX_Monsters/FX_Monster_Troll/death/P_TrollDeathImpact.P_TrollDeathImpact" HitLocation))

(event Custom|Server_Bite
  (bind _bitecollision (Variables|Default|GetBiteCollision))
  (bind _overlappingactors (Collision|GetOverlappingActors _bitecollision "/Game/PlayerCharacter/Player.Player_C" :!class /Script/Engine.PrimitiveComponent))
  (bind _output (Utilities|Array|Get(acopy) _overlappingactors))
  ;[1 1 1] Server - Bite
  (Utilities|IsValid _output
    (:Is%20Valid
      (Default|TakeDamage (.AsPlayer (Utilities|Casting|CastToPlayer _output)) (Math|Float|MakeLiteralFloat 25.0)))))

(event Custom|RecoverHealth
  ;[1 1 1] Health Recovery
  (Math|Float|IncrementFloat (Variables|Default|GetHealth)))

(event EventBeginPlay
  (bind _healthrecoveryrate (Variables|Default|GetHealthRecoveryRate))
  ;[1 1 1] Health Recovery
  (if (> _healthrecoveryrate 0.0)
    (Utilities|Time|SetTimerbyEvent (delegate Custom|RecoverHealth) (/ 1.0 _healthrecoveryrate) true)))

(event Collision|EventActorBeginOverlap
  (params (OtherActor :type Actor%20Object%20Reference)))

(event EventTick
  (params (DeltaSeconds :type Float%20%28single-precision%29)))

(fn ConstructionScript
  ;[1 1 1] Load Data From EnemiesTable
  (|CallParentFunction)
  (bind _returnvalue (Utilities|GetDataTableRow "/Game/GameplayData/EnemiesTable.EnemiesTable" "TypeA")
    (:then
      (Variables|Default|SetHealth (.MaxHealth (Utilities|Struct|BreakEnemyStatsStruct _returnvalue)))
      (Variables|/Script/Engine.CharacterMovementComponent|SetMaxWalkSpeed (Variables|Character|GetCharacterMovement) (.Speed (Utilities|Struct|BreakEnemyStatsStruct _returnvalue)))
      (Variables|Default|SetBiteDistance (.BiteDistance (Utilities|Struct|BreakEnemyStatsStruct _returnvalue)))
      (Variables|Default|SetHealthRecoveryRate (.HealthRecoveryRate (Utilities|Struct|BreakEnemyStatsStruct _returnvalue))))
    (:RowNotFound)))