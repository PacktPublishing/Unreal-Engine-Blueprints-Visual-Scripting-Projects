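; Functional test that checks the player pawn gets destroyed when falling rather than continuing to exist below the level.
; IsReady holds the test until player pawn 0 is valid.
; Tick then fails the test if the pawn drops below a fixed Z threshold, or succeeds once the pawn is no longer valid.
; Either result quits the game right after finishing the test.
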(event EventPrepareTest)

(event EventStartTest)

(event EventTick
  (params (DeltaSeconds :type Float%20%28single-precision%29))
  ;[1 1 1] Functional Test - If player still exists below a certain z, then the test fails; if the player gets destroyed at a certain point, then the test succeeds
  (Utilities|IsValid (Game|Player|GetPlayerPawn 0)
    (:Is%20Valid
      (if (< (.z (Transformation|GetActorLocation (Game|Player|GetPlayerPawn 0))) -6e+02)
        (Class|FunctionalTest|FinishTest "Failed")
        (Game|QuitGame 0 "Quit" :!label _label)))
    (:Is%20Not%20Valid
      (Class|FunctionalTest|FinishTest "Succeeded" "Test Succeeded")
      (goto _label))))

(fn ConstructionScript)

(fn IsReady
  ;[1 1 1] Check if the Player Pawn is available in order to run this test.
  (return (Utilities|IsValid (Game|Player|GetPlayerPawn 0))))