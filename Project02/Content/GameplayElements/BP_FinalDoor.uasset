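; BP_FinalDoor is a door that destroys itself to open once every BP_CollectableItem in the map has been collected.
; On BeginPlay it counts the items, caches all BP_FillingStatue actors and opens at once if the map has no items.
; Each ItemCollected call decrements the remaining count, sets every statue's fill to the collected fraction, and triggers OpenDoor at zero.
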(event Custom|OpenDoor
  ;[1 1 1] Open Door Event
  (Actor|DestroyActor))

(event Custom|ItemCollected
  ;[1 1 1] An item has been collected, check if all of them are, if true open the door
  (bind _result (Math|Integer|DecrementInt (Variables|Default|GetRemainingCollectableItems))
    (:%20%20
      (CallFunction|UpdateFillingStatues)
      (if (== _result 0)
        (CallFunction|OpenDoor)))))

(event EventBeginPlay
  ;[1 1 1] Check How many Collectable Items there are in the map
  (bind _outactors (Actor|GetAllActorsOfClass "/Game/GameplayElements/BP_FillingStatue.BP_FillingStatue_C"))
  (Variables|Default|SetFillingStatues _outactors)
  (bind _outactors_2 (Actor|GetAllActorsOfClass "/Game/GameplayElements/BP_CollectableItem.BP_CollectableItem_C"))
  (bind _output_get (Variables|Default|SetRemainingCollectableItems (Utilities|Array|Length _outactors_2)))
  (bind _output_get_2 (Variables|Default|SetTotalNumberOfItems _output_get))
  (CallFunction|UpdateFillingStatues)
  (if (== _output_get_2 0)
    (CallFunction|OpenDoor)))

(event Collision|EventActorBeginOverlap
  (params (OtherActor :type Actor%20Object%20Reference)))

(event EventTick
  (params (DeltaSeconds :type Float%20%28single-precision%29)))

(fn ConstructionScript)

(fn UpdateFillingStatues
  ;[1 1 1] Update Filling Statues
  (for _array_element (Variables|Default|GetFillingStatues)
    (Default|SetFillingValue _array_element (- 1.0 (/ (Math|Conversions|ToFloat(Integer) (Variables|Default|GetRemainingCollectableItems)) (Math|Conversions|ToFloat(Integer) (Variables|Default|GetTotalNumberOfItems)))))))