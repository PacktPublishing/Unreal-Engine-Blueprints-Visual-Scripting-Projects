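; BP_DynamicLight is an actor that lights up and shifts color based on the player character's proximity.
; It adds a point light component at BeginPlay rather than placing one in the component tree.
; Each Tick it hides the light beyond an activation distance; within it, the color lerps from begin to end color as the player moves inside the color-change threshold, scaled by a second distance.
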(event EventBeginPlay
  ;[1 1 1] Creating a Dynamic Light
  (bind _returnvalue (AddComponent|AddPointLightComponent false))
  (Variables|Default|SetPointLight _returnvalue))

(event Collision|EventActorBeginOverlap
  (params (OtherActor :type Actor%20Object%20Reference)))

(event EventTick
  (params (DeltaSeconds :type Float%20%28single-precision%29))
  (bind _pointlight (Variables|Default|GetPointLight))
  ;[1 1 1] Implementation of the Logic
  (if (> (Transformation|GetDistanceTo (Game|GetPlayerCharacter 0)) (Variables|Default|GetDistanceForActivation))
    (Rendering|SetVisibility _pointlight false false)
    (else
      (Rendering|SetVisibility _pointlight true false)
      (Rendering|Components|Light|SetLightColor (Variables|Default|GetPointLight) (Math|Color|Lerp(LinearColor) (Variables|Default|GetBeginColor) (Variables|Default|GetEndColor) (/ (Math|Float|Absolute(Float) (Math|Float|Min(Float) (- (Transformation|GetDistanceTo (Game|GetPlayerCharacter 0)) (Variables|Default|GetDistanceBeginChangeColor)) 0.0)) (Variables|Default|GetDistanceEndChangeColor))) true))))

(fn ConstructionScript)