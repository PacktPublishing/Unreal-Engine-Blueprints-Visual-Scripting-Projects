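; BP_FillingStatue is a statue actor whose material shows a variable fill level.
; The construction script creates a dynamic instance of MI_FillingMaterial on the static mesh and starts it empty.
; SetFillingValue multiplies the given fraction by the actor's bounds height, divides by Z scale, writes the result to the FillingValue parameter, and prints it to screen.
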(event Custom|Set%20Filling%20Value
  (params (FillingValueInPercentage :type Float%20%28single-precision%29))
  (bind _returnvalue (Transformation|GetActorTransform))
  (bind _boxextent (Collision|GetActorBounds false))
  (bind _returnvalue_2 (* FillingValueInPercentage (.z _boxextent) 2.0))
  (bind _returnvalue_3 (/ _returnvalue_2 (.z (.scale _returnvalue))))
  (Rendering|Material|SetScalarParameterValue (Variables|Default|GetDynamicMaterial) "FillingValue" _returnvalue_3 :!class /Script/Engine.MaterialInstanceDynamic)
  (Development|PrintString (Utilities|String|ToString(Float) _returnvalue_3)))

(event EventBeginPlay)

(event Collision|EventActorBeginOverlap
  (params (OtherActor :type Actor%20Object%20Reference)))

(event EventTick
  (params (DeltaSeconds :type Float%20%28single-precision%29)))

(fn ConstructionScript
  (bind _returnvalue (Rendering|Material|CreateDynamicMaterialInstance (Variables|Default|GetStaticMesh) 0 "/Game/Materials/MI_FillingMaterial.MI_FillingMaterial" "None" :!class /Script/Engine.PrimitiveComponent))
  (Variables|Default|SetDynamicMaterial _returnvalue)
  (CallFunction|SetFillingValue 0.0))